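; Blueprint helper library that remaps PSN tracker data between axis conventions.
; PSN XYZ Swapper offsets then scales position, target position and orientation, then swaps chosen axis pairs, with separate modes for location and rotation.
; Speed and acceleration follow the location swap without offset or scaling, and status passes through unchanged.
; PSN MA Preset wraps the swapper with an XY location swap, leaving other settings at their defaults.
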(fn PSNXYZSwapper
  (params (PSNTrackerData :type PSN%20Tracker%20Data%20Structure%20%28by%20ref%29) (LocationSwap :type XYZSwapOptions%20Enum :default "NewEnumerator3") (RotationSwap :type XYZSwapOptions%20Enum :default "NewEnumerator3") (UE%20LocationOffset%20in%20'cm'%20Default=0 :type Vector) (UE%20OrientationOffset%20in%20'degrees'%20Default=0 :type Rotator) (ScaleLocationFactor%20Default=1 :type Vector :default "1.000000,1.000000,1.000000") (ScaleOrientationFactor%20Default=1 :type Float%20%28single-precision%29))
  (bind (_position _speed _orientation _status _acceleration _targetposition) (Utilities|Struct|BreakPSNTrackerData PSNTrackerData))
  (LocalVariables|SetPosition (* (+ UE%20LocationOffset%20in%20'cm'%20Default=0 _position) ScaleLocationFactor%20Default=1))
  (LocalVariables|SetSpeed _speed)
  (LocalVariables|SetOrientation (* (Math|Rotator|CombineRotators _orientation UE%20OrientationOffset%20in%20'degrees'%20Default=0) ScaleOrientationFactor%20Default=1))
  (LocalVariables|SetAcceleration _acceleration)
  (LocalVariables|SetTarget%20Position (* (+ UE%20LocationOffset%20in%20'cm'%20Default=0 _targetposition) ScaleLocationFactor%20Default=1))
  (LocalVariables|SetLocationSwapLoc LocationSwap)
  (LocalVariables|SetRotationSwapLoc RotationSwap)
  (return (Utilities|Struct|MakePSNTrackerData (Utilities|Select :Index (LocalVariables|GetLocationSwapLoc) :NewEnumerator3 (LocalVariables|GetPosition) :NewEnumerator1 (Math|Vector|MakeVector (.Z (Math|Vector|BreakVector (LocalVariables|GetPosition))) (.Y (Math|Vector|BreakVector (LocalVariables|GetPosition))) (.X (Math|Vector|BreakVector (LocalVariables|GetPosition)))) :NewEnumerator0 (Math|Vector|MakeVector (.Y (Math|Vector|BreakVector (LocalVariables|GetPosition))) (.X (Math|Vector|BreakVector (LocalVariables|GetPosition))) (.Z (Math|Vector|BreakVector (LocalVariables|GetPosition)))) :NewEnumerator2 (Math|Vector|MakeVector (.X (Math|Vector|BreakVector (LocalVariables|GetPosition))) (.Z (Math|Vector|BreakVector (LocalVariables|GetPosition))) (.Y (Math|Vector|BreakVector (LocalVariables|GetPosition))))) (Utilities|Select :Index (LocalVariables|GetLocationSwapLoc) :NewEnumerator3 (LocalVariables|GetSpeed) :NewEnumerator1 (Math|Vector|MakeVector (.Z (Math|Vector|BreakVector (LocalVariables|GetSpeed))) (.Y (Math|Vector|BreakVector (LocalVariables|GetSpeed))) (.X (Math|Vector|BreakVector (LocalVariables|GetSpeed)))) :NewEnumerator0 (Math|Vector|MakeVector (.Y (Math|Vector|BreakVector (LocalVariables|GetSpeed))) (.X (Math|Vector|BreakVector (LocalVariables|GetSpeed))) (.Z (Math|Vector|BreakVector (LocalVariables|GetSpeed)))) :NewEnumerator2 (Math|Vector|MakeVector (.X (Math|Vector|BreakVector (LocalVariables|GetSpeed))) (.Z (Math|Vector|BreakVector (LocalVariables|GetSpeed))) (.Y (Math|Vector|BreakVector (LocalVariables|GetSpeed))))) (Utilities|Select :Index (LocalVariables|GetRotationSwapLoc) :NewEnumerator3 (LocalVariables|GetOrientation) :NewEnumerator1 (Math|Rotator|MakeRotator (.Yaw (Math|Rotator|BreakRotator (LocalVariables|GetOrientation))) (.Pitch (Math|Rotator|BreakRotator (LocalVariables|GetOrientation))) (.Roll (Math|Rotator|BreakRotator (LocalVariables|GetOrientation)))) :NewEnumerator0 (Math|Rotator|MakeRotator (.Pitch (Math|Rotator|BreakRotator (LocalVariables|GetOrientation))) (.Roll (Math|Rotator|BreakRotator (LocalVariables|GetOrientation))) (.Yaw (Math|Rotator|BreakRotator (LocalVariables|GetOrientation)))) :NewEnumerator2 (Math|Rotator|MakeRotator (.Roll (Math|Rotator|BreakRotator (LocalVariables|GetOrientation))) (.Yaw (Math|Rotator|BreakRotator (LocalVariables|GetOrientation))) (.Pitch (Math|Rotator|BreakRotator (LocalVariables|GetOrientation))))) _status (Utilities|Select :Index (LocalVariables|GetLocationSwapLoc) :NewEnumerator3 (LocalVariables|GetAcceleration) :NewEnumerator1 (Math|Vector|MakeVector (.Z (Math|Vector|BreakVector (LocalVariables|GetAcceleration))) (.Y (Math|Vector|BreakVector (LocalVariables|GetAcceleration))) (.X (Math|Vector|BreakVector (LocalVariables|GetAcceleration)))) :NewEnumerator0 (Math|Vector|MakeVector (.Y (Math|Vector|BreakVector (LocalVariables|GetAcceleration))) (.X (Math|Vector|BreakVector (LocalVariables|GetAcceleration))) (.Z (Math|Vector|BreakVector (LocalVariables|GetAcceleration)))) :NewEnumerator2 (Math|Vector|MakeVector (.X (Math|Vector|BreakVector (LocalVariables|GetAcceleration))) (.Z (Math|Vector|BreakVector (LocalVariables|GetAcceleration))) (.Y (Math|Vector|BreakVector (LocalVariables|GetAcceleration))))) (Utilities|Select :Index (LocalVariables|GetLocationSwapLoc) :NewEnumerator3 (LocalVariables|GetTarget%20Position) :NewEnumerator1 (Math|Vector|MakeVector (.Z (Math|Vector|BreakVector (LocalVariables|GetTarget%20Position))) (.Y (Math|Vector|BreakVector (LocalVariables|GetTarget%20Position))) (.X (Math|Vector|BreakVector (LocalVariables|GetTarget%20Position)))) :NewEnumerator0 (Math|Vector|MakeVector (.Y (Math|Vector|BreakVector (LocalVariables|GetTarget%20Position))) (.X (Math|Vector|BreakVector (LocalVariables|GetTarget%20Position))) (.Z (Math|Vector|BreakVector (LocalVariables|GetTarget%20Position)))) :NewEnumerator2 (Math|Vector|MakeVector (.X (Math|Vector|BreakVector (LocalVariables|GetTarget%20Position))) (.Z (Math|Vector|BreakVector (LocalVariables|GetTarget%20Position))) (.Y (Math|Vector|BreakVector (LocalVariables|GetTarget%20Position))))))))

(fn PSNMAPreset
  (params (PSNTrackerData :type PSN%20Tracker%20Data%20Structure%20%28by%20ref%29))
  (return (CallFunction|PSNXYZSwapper PSNTrackerData "NewEnumerator0" "NewEnumerator3" "0, 0, 0" "0, 0, 0" "1.000000,1.000000,1.000000" 1.0)))